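; Player controller for gameplay that runs the HUD, pause menu and game-over screen.
; StartLogic retries until it possesses a BP_Pawn, then outside the start and end levels adds W_GameMain, binds pawn events for lives, score and losing, and creates a save object.
; Escape pauses with W_Pause for resume or quit.
; Losing pauses with W_GameOver and a sound; its restart handler only removes the widget, while exit quits.
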(event `StartLogic`
  (bind _gamewidget (`self.GameWidget`))
  (bind _asbp_pawn (cast `/Game/Blueprints/Player/BP_Pawn` (`self.K2_GetPawn`) :!label _label)
    (:`then`
      (set `self.BP_Pawn` _asbp_pawn)
      (`/Engine/EditorBlueprintResources/StandardMacros.IsValid` _gamewidget
        (:`Is Valid`
          (if (`Widget.IsInViewport` _gamewidget)
            (`Widget.RemoveFromParent` _gamewidget)))
        (:`Is Not Valid`
          _))
      (bind _returnvalue (`GameplayStatics.GetCurrentLevelName` true))
      (if (and (`KismetStringLibrary.NotEqual_StrStr` _returnvalue "GameStart") (`KismetStringLibrary.NotEqual_StrStr` _returnvalue "GameEnd"))
        (bind _returnvalue_2 (`|CreateWidget` "/Game/UI/W_GameMain.W_GameMain_C" (`GameplayStatics.GetPlayerController` 0)))
        (bind _output_get (set `self.GameWidget` _returnvalue_2))
        (`UserWidget.AddToViewport` _output_get 0)
        (`self.Part2`)))
    (:`CastFailed`
      (`KismetSystemLibrary.Delay` 0.2)
      (goto _label))))

(event `Part2`
  (bind _bp_pawn (`self.BP_Pawn`))
  (add `PlayerPawn.Looser` _bp_pawn (delegate `ShowGameOver`))
  (add `PlayerPawn.ChangeLife` _bp_pawn (delegate `UpdateLives`))
  (add `PlayerPawn.ScoreChanged` _bp_pawn (delegate `ScoreChanged_Event`))
  (bind _returnvalue (`GameplayStatics.CreateSaveGameObject` "/Game/Blueprints/Game/BP_SaveGame.BP_SaveGame_C"))
  (set `self.As BP Save Game` _returnvalue)
  (`self.WidgetDone`))

(event `ShowGameOver`
  (`self.GameOver`))

(event `UpdateLives`
  (`/Game/UI/W_GameMain.FillLives` (`self.GameWidget`) (`PlayerPawn.RemainingLife` (`self.BP_Pawn`))))

(event `ScoreChanged_Event`
  (params (Score :type Integer))
  (`/Engine/EditorBlueprintResources/StandardMacros.IsValid` (`self.GameWidget`) :!label _label_2
    (:`Is Valid`
      (`/Game/UI/W_GameMain.UpdateCurrentScore` (`self.GameWidget`) Score))
    (:`Is Not Valid`
      (`KismetSystemLibrary.Delay` 0.2)
      (goto _label_2))))

(event `Key|Shift+Escape`
  (params (Key :type "Key Structure"))
  (bind _w_pause (`self.W_Pause`))
  ;[0 0 0] Paused
  (:`Pressed`
    (`GameplayStatics.SetGamePaused` true :!label _label_3)
    (bind _returnvalue (`|CreateWidget` "/Game/UI/W_Pause.W_Pause_C" self))
    (bind _output_get (set `self.W_Pause` _returnvalue))
    (`UserWidget.AddToViewport` _output_get 0)
    (set `self.bShowMouseCursor` true)
    (`WidgetBlueprintLibrary.SetInputMode_UIOnlyEx` self null)
    (add `/Game/UI/W_Pause.ConfirmExit` _w_pause (delegate `ConfirmExit_Event_0`))
    (add `/Game/UI/W_Pause.ResumeGame` _w_pause (delegate `ResumeGame_Event_0`))))

(event `Key|Escape`
  (params (Key :type "Key Structure"))
  ;[0 0 0] Paused
  (:`Pressed`
    (goto _label_3)))

(event `ConfirmExit_Event_0`
  ;[0 0 0] Paused
  (`Widget.RemoveFromParent` (`self.W_Pause`))
  (`KismetSystemLibrary.QuitGame` null "Quit"))

(event `ResumeGame_Event_0`
  ;[0 0 0] Paused
  (remove `/Game/UI/W_Pause.ResumeGame` (`self.W_Pause`) (delegate `ResumeGame_Event_0`))
  (`Widget.RemoveFromParent` (`self.W_Pause`))
  (set `self.bShowMouseCursor` false)
  (`WidgetBlueprintLibrary.SetInputMode_GameOnly` self)
  (`GameplayStatics.SetGamePaused` false))

(event `GameOver`
  (bind _gameoverw (`self.GameOverW`))
  ;[0 0 0] GAME OVER
  (`GameplayStatics.SetGamePaused` true)
  (set `self.bShowMouseCursor` true)
  (bind _returnvalue (`|CreateWidget` "/Game/UI/W_GameOver.W_GameOver_C" (`GameplayStatics.GetPlayerController` 0)))
  (bind _output_get (set `self.GameOverW` _returnvalue))
  (`UserWidget.AddToViewport` _output_get 0)
  (`GameplayStatics.PlaySound2D` (`self.SoundLooser`) 1.0 1.0 0.0 null null)
  (`WidgetBlueprintLibrary.SetInputMode_UIOnlyEx` (`GameplayStatics.GetPlayerController` 0) (`self.GameOverW`))
  (add `/Game/UI/W_GameOver.RestartClicked` _gameoverw (delegate `RestartClicked_Event_0`))
  (add `/Game/UI/W_GameOver.ExitClicked` _gameoverw (delegate `ExitClicked_Event`)))

(event `RestartClicked_Event_0`
  (bind _gameoverw (`self.GameOverW`))
  ;[0 0 0] GAME OVER
  (remove `/Game/UI/W_GameOver.RestartClicked` _gameoverw (delegate `RestartClicked_Event_0`))
  (`Widget.RemoveFromParent` _gameoverw))

(event `ExitClicked_Event`
  (bind _gameoverw (`self.GameOverW`))
  ;[0 0 0] GAME OVER
  (remove `/Game/UI/W_GameOver.ExitClicked` _gameoverw (delegate `ExitClicked_Event`))
  (`Widget.RemoveFromParent` _gameoverw)
  (`KismetSystemLibrary.QuitGame` null "Quit"))

(fn `UserConstructionScript`)