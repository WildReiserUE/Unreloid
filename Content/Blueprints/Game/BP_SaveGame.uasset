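; Save game object that carries record score and remaining lives between levels through named save slots.
; CheckSave loads the previous level's slot from level two onward, otherwise the given slot, creating one on the first level if absent.
; LoadFromSlot pushes saved values into the player pawn and game widget, then deletes that slot.
; SaveRecord retains the higher score and saves the player controller's save object.
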(event Custom|LoadPrevLelel
  (params (PrevLevel :type String) (CurLevel :type String))
  (bind _pcgame (Variables|Default|GetPCGame))
  (bind _as_bp_save_game (Variables|/Game/Blueprints/Game/PC_Game.PC_Game_C|GetAs%20BP%20Save%20Game _pcgame))
  (bind _returnvalue (SaveGame|DoesSaveGameExist PrevLevel))
  (if _returnvalue
    (CallFunction|LoadfromSlot PrevLevel)
    (else
      (Variables|BP_SaveGame_C|SetRecordScore _as_bp_save_game (Variables|Default|GetRecordScore))
      (Variables|BP_SaveGame_C|SetRemainLife _as_bp_save_game (Variables|/Script/Arcanoid.PlayerPawn|GetRemainingLife (Variables|/Game/Blueprints/Game/PC_Game.PC_Game_C|GetBP_Pawn _pcgame)))
      (bind _returnvalue_2 (SaveGame|SaveGametoSlot _as_bp_save_game CurLevel))
      (if _returnvalue_2
        (Development|PrintString 0 "CREATE PREV SAVE SUCCESS" true true "(R=0.000000,G=1.000000,B=0.000000,A=1.000000)")
        (CallFunction|LoadfromSlot CurLevel)
        (else
          (Development|PrintString 0 "CREATE SAVE FAIL" true true "(R=1.000000,G=0.000000,B=0.000000,A=1.000000)"))))))

(event Custom|CheckSave
  (params (SaveName :type String) (PCGame :type PC%20Game%20Object%20Reference) (RealLevel :type String) (LevelIndex :type Integer))
  (bind _returnvalue (- LevelIndex 1))
  (bind _returnvalue_2 (Utilities|String|ToString(Integer) _returnvalue))
  (bind _returnvalue_3 (Utilities|String|Append RealLevel _returnvalue_2))
  (Variables|Default|SetPCGame PCGame)
  (if (>= LevelIndex 2)
    (Development|PrintString 0 "TRUE LOGIC")
    (CallFunction|LoadPrevLelel _returnvalue_3)
    (else
      (bind _returnvalue_4 (SaveGame|DoesSaveGameExist SaveName))
      (if _returnvalue_4
        (Development|PrintString 0 "LOADING AFTER CHECK")
        (CallFunction|LoadfromSlot SaveName)
        (else
          (Variables|BP_SaveGame_C|SetRecordScore (Variables|/Game/Blueprints/Game/PC_Game.PC_Game_C|GetAs%20BP%20Save%20Game (Variables|Default|GetPCGame)) (Variables|Default|GetRecordScore))
          (Variables|BP_SaveGame_C|SetRemainLife (Variables|/Game/Blueprints/Game/PC_Game.PC_Game_C|GetAs%20BP%20Save%20Game (Variables|Default|GetPCGame)) (Variables|/Script/Arcanoid.PlayerPawn|GetRemainingLife (Variables|/Game/Blueprints/Game/PC_Game.PC_Game_C|GetBP_Pawn (Variables|Default|GetPCGame))))
          (CallFunction|LoadPrevLelel _returnvalue_3 SaveName))))))

(event Custom|SaveRecord
  (params (SlotName :type String) (Score :type Integer) (RemainLife :type Integer))
  (Variables|Default|SetRemainLife RemainLife)
  (bind _returnvalue (SaveGame|DoesSaveGameExist SlotName))
  (if _returnvalue
    (bind _returnvalue_2 (SaveGame|LoadGamefromSlot SlotName))
    (bind _asbp_save_game (Utilities|Casting|CastToBP_SaveGame _returnvalue_2)))
  (if (> Score (Variables|Default|GetRecordScore))
    (Variables|Default|SetRecordScore Score)
    (else
      (Variables|Default|SetRecordScore (Variables|Default|GetRecordScore))))
  (bind _returnvalue_3 (SaveGame|SaveGametoSlot (Variables|/Game/Blueprints/Game/PC_Game.PC_Game_C|GetAs%20BP%20Save%20Game (Variables|Default|GetPCGame)) SlotName))
  (if _returnvalue_3
    (Development|PrintString 0 "SAVE DONE")
    (else
      (Development|PrintString 0 "SAVE FAIL"))))

(event Custom|LoadFromSlot
  (params (SlotName :type String))
  (bind _pcgame (Variables|Default|GetPCGame))
  (bind _bp_pawn (Variables|/Game/Blueprints/Game/PC_Game.PC_Game_C|GetBP_Pawn _pcgame))
  (bind _gamewidget (Variables|/Game/Blueprints/Game/PC_Game.PC_Game_C|GetGameWidget _pcgame))
  (bind _returnvalue (SaveGame|LoadGamefromSlot SlotName))
  (Utilities|IsValid _returnvalue
    (:Is%20Valid
      (bind _asbp_save_game (Utilities|Casting|CastToBP_SaveGame _returnvalue))
      (bind _output_get (Variables|/Script/Arcanoid.PlayerPawn|SetPlayerScore _bp_pawn (Variables|BP_SaveGame_C|GetRecordScore _asbp_save_game)))
      (Default|UpdateCurrentScore _gamewidget _output_get)
      (Default|UpdateRecord _gamewidget (Variables|BP_SaveGame_C|GetRecordScore _asbp_save_game))
      (bind _output_get_2 (Variables|/Script/Arcanoid.PlayerPawn|SetRemainingLife _bp_pawn (Variables|BP_SaveGame_C|GetRemainLife _asbp_save_game)))
      (Default|FillLives _gamewidget _output_get_2)
      (Development|PrintString 0 "LOADING END")
      (SaveGame|DeleteGameinSlot SlotName))))